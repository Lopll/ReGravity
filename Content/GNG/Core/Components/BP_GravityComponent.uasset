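; Actor component giving its owner custom gravity that can be redirected, suspended for hovering, or turned into a spin.
; Tick sends gravity and spin forces through owner messages and resets to default direction when ShouldStopGravityEffect passes.
; Gameplay tags track Changed, Hovering and Spinning states; enough detected hits trigger a timed spin with hover.
; Helpers swap overlay materials, test walkable surfaces against gravity and report scaled speed.
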(event `self.ReceiveBeginPlay`
  (`KismetSystemLibrary.Delay` 2.0)
  (`/Engine/EditorBlueprintResources/StandardMacros.IsValid` (`self.PhysicBase`)
    (:`Is Not Valid`
      (`KismetSystemLibrary.PrintString` "WARNING: PhysBase is None" true true (struct :`R` 1.0 :`G` 0.00016 :`B` 0.042168 :`A` 1.0)))))

(event `self.ReceiveTick`
  (params (DeltaSeconds :type "Float (single-precision)"))
  (`|ExecutionSequence`
    (:`then_0`
      ; Apply Gravity
      (if (`self.bGravityEnabled`)
        (message `/Game/GNG/Core/Interfaces/BPI_GravityChangable.ApplyForce` (`self.GetOwner`) (`self.PhysicBase`) (`self.GravityDir`) (`self.G`) DeltaSeconds)))
    (:`then_1`
      ; Reset Gravity
      (if (`self.ShouldStopGravityEffect`)
        (`self.ResetGravity`)))
    (:`then_3`
      ; Spin
      (if (`BlueprintGameplayTagLibrary.HasTag` (`self.GameplayTagContainer`) (struct :`TagName` "Gravity.Spinning") true)
        (message `/Game/GNG/Core/Interfaces/BPI_GravityChangable.AddTorque` (`self.GetOwner`) (* (`SceneComponent.GetUpVector` (`self.PhysicBase`)) (`self.SpinRotateSpeed`)) true)
        (message `/Game/GNG/Core/Interfaces/BPI_GravityChangable.ApplyForce` (`self.GetOwner`) (`self.PhysicBase`) (`self.SpinDir`) (`self.SpinMoveSpeed`) DeltaSeconds)))))

(event `Hover`
  (`self.StartHover`)
  (`KismetSystemLibrary.Delay` (`self.HoverTime`))
  (`self.StopHover`))

(event `HitDetected`
  (params (SpinDir :type "Vector Structure"))
  (if (not (`BlueprintGameplayTagLibrary.HasTag` (`self.GameplayTagContainer`) (struct :`TagName` "Gravity.Spinning") true))
    (bind _result (`/Engine/EditorBlueprintResources/StandardMacros.IncrementInt` (`self.HitsCounter`))
      (:`  `
        (if (>= _result (`self.HITS_FOR_SPINNING`))
          (`|ExecutionSequence`
            (:`then_0`
              (set `self.HitsCounter` 0)
              (`BlueprintGameplayTagLibrary.AddGameplayTag` (`self.GameplayTagContainer`) (struct :`TagName` "Gravity.Spinning"))
              (set `self.SpinDir` SpinDir)
              (`self.StartHover`))
            (:`then_1`
              (`KismetSystemLibrary.Delay` (`self.SpinTime`))
              (`BlueprintGameplayTagLibrary.RemoveGameplayTag` (`self.GameplayTagContainer`) (struct :`TagName` "Gravity.Spinning"))
              (`self.StopHover`))))))))

(fn `ChangeGravity`
  (params (GravityDir :type "Vector Structure") (bIsGravityChanged :type Boolean))
  (set `self.GravityDir` GravityDir)
  (`BlueprintGameplayTagLibrary.RemoveGameplayTag` (`self.GameplayTagContainer`) (struct :`TagName` "Gravity.Hovering"))
  (set `self.bGravityEnabled` true)
  (if (`local.bIsGravityChanged`)
    (`BlueprintGameplayTagLibrary.AddGameplayTag` (`self.GameplayTagContainer`) (struct :`TagName` "Gravity.Changed"))
    (else
      (`BlueprintGameplayTagLibrary.RemoveGameplayTag` (`self.GameplayTagContainer`) (struct :`TagName` "Gravity.Changed")))))

(fn `GetVelocity`
  (returns (Velocity :type "Float (double-precision)"))
  (return (* (`KismetMathLibrary.VSize` (`Actor.GetVelocity` (`self.GetOwner`))) 0.01)))

(fn `IsWalkableSurface`
  (params (CollisionProfileName :type Name) (`-Normal` :type "Vector Structure"))
  (returns (Result :type Boolean))
  (locals (RelativelyCloseThreshold :type "Float (double-precision)" :default 0.3))
  (return (and (or (== CollisionProfileName "BlockAll") (== CollisionProfileName "BlockAllDynamic")) (> (`KismetMathLibrary.Dot_VectorVector` `-Normal` (`self.GravityDir`)) (`local.RelativelyCloseThreshold`)))))

(fn `ResetGravity`
  (set `self.GravityDir` (`self.DefaultGravityDir`))
  (set `self.bGravityEnabled` true)
  (`BlueprintGameplayTagLibrary.RemoveGameplayTag` (`self.GameplayTagContainer`) (struct :`TagName` "Gravity.Changed"))
  (`BlueprintGameplayTagLibrary.RemoveGameplayTag` (`self.GameplayTagContainer`) (struct :`TagName` "Gravity.Spinning"))
  (set `self.HitsCounter` 0))

(fn `SetOverlayMaterial`
  (params (NewOverlayMaterial :type "MaterialInterface Object Reference"))
  (if (`self.bMaterialChangeEnabled`)
    (bind _asmesh_component (cast `MeshComponent` (`self.PhysicBase`))
      (:`then`
        (`MeshComponent.SetOverlayMaterial` _asmesh_component NewOverlayMaterial))
      (:`CastFailed`
        (`MeshComponent.SetOverlayMaterial` (`self.MeshComponent`) NewOverlayMaterial)))))

(fn `StartHover`
  (locals (`-G` :type "Vector Structure"))
  (bind _returnvalue (`self.GetOwner`))
  (bind _returnvalue_2 (`KismetMathLibrary.Conv_IntToDouble` (* (- (`KismetMathLibrary.RandomInteger` 3) 1) (`self.HoverStrength`))))
  (bind _output_get (set `local.-G` (* (`self.GravityDir`) -1)))
  (message `/Game/GNG/Core/Interfaces/BPI_GravityChangable.ApplyForce` _returnvalue (`self.PhysicBase`) _output_get (`self.HoverStrength`) (`GameplayStatics.GetWorldDeltaSeconds`))
  (message `/Game/GNG/Core/Interfaces/BPI_GravityChangable.ApplyForceAtLocalLocation` _returnvalue (`self.PhysicBase`) (`local.-G`) (`self.HoverStrength`) (`KismetMathLibrary.MakeVector` _returnvalue_2 _returnvalue_2 _returnvalue_2))
  (set `self.bGravityEnabled` false)
  (`BlueprintGameplayTagLibrary.AddGameplayTag` (`self.GameplayTagContainer`) (struct :`TagName` "Gravity.Hovering"))
  (message `/Game/GNG/Core/Interfaces/BPI_GravityChangable.OnHoverStart` (`self.GetOwner`)))

(fn `StopHover`
  (bind _gameplaytagcontainer (`self.GameplayTagContainer`))
  (if (and (`BlueprintGameplayTagLibrary.HasTag` _gameplaytagcontainer (struct :`TagName` "Gravity.Hovering") true) (not (`BlueprintGameplayTagLibrary.HasTag` _gameplaytagcontainer (struct :`TagName` "Gravity.Spinning") true)))
    (set `self.bGravityEnabled` true)
    (`BlueprintGameplayTagLibrary.RemoveGameplayTag` (`self.GameplayTagContainer`) (struct :`TagName` "Gravity.Hovering"))
    (message `/Game/GNG/Core/Interfaces/BPI_GravityChangable.OnHoverEnd` (`self.GetOwner`))))