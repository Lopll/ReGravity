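; Physics object with health whose gravity can be changed, taking and dealing impact damage.
; Implements BPI_GravityChangable for force, torque and hover particles, delegating gravity state to BPGravityComponent.
; While moving under non-default gravity, hits on new walkable surfaces realign gravity and self-damage; other hits damage non-player HP owners by spin or momentum.
; Damage reduces HPComp health; player hits while hovering also notify the gravity component.
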(event `self.ReceiveBeginPlay`
  (set `/Game/GNG/Core/Components/BP_GravityComponent.PhysicBase` (`self.StaticMesh`) (`self.BP_GravityComponent`))
  (add `self.OnTakeAnyDamage` (`|CreateDelegate` :!event `OnAnyDamage`))
  (bind _output_get (set `HPComponent.MAX_HP` (`self.MaxHP`) (`self.HPComp`)))
  (`HPComponent.SetHP` (`self.HPComp`) _output_get)
  (set `self.FallDamageLimit` (* (/ (`self.FallDamageLimit`) 100.0) (`HPComponent.MAX_HP` (`self.HPComp`)))))

(event `/Game/GNG/Core/Interfaces/BPI_GravityChangable.ApplyForce`
  (params (PhysComponent :type "PrimitiveComponent Object Reference") (ForceDirection :type "Vector Structure") (ForceStrength :type "Float (double-precision)") (DeltaTime :type "Float (double-precision)"))
  (`PrimitiveComponent.AddForce` PhysComponent (* ForceDirection ForceStrength) "None" true))

(event `/Game/GNG/Core/Interfaces/BPI_GravityChangable.ApplyForceAtLocalLocation`
  (params (PhysComponent :type "PrimitiveComponent Object Reference") (ForceDirection :type "Vector Structure") (ForceStrength :type "Float (double-precision)") (LocalLocation :type "Vector Structure"))
  (`PrimitiveComponent.AddForceAtLocationLocal` PhysComponent (* ForceDirection ForceStrength) LocalLocation "None"))

(event `/Game/GNG/Core/Interfaces/BPI_GravityChangable.AddTorque`
  (params (Torque :type "Vector Structure") (AccelChange :type Boolean))
  (`PrimitiveComponent.AddTorqueInDegrees` (`self.StaticMesh`) Torque "None" AccelChange))

(event `/Game/GNG/Core/Interfaces/BPI_GravityChangable.OnHoverStart`
  (`ActorComponent.Activate` (`self.Niagara`) true))

(event `/Game/GNG/Core/Interfaces/BPI_GravityChangable.OnHoverEnd`
  (`ActorComponent.Deactivate` (`self.Niagara`)))

(event `self.StaticMesh.OnComponentHit`
  (params (HitComponent :type "PrimitiveComponent Object Reference") (OtherActor :type "Actor Object Reference") (OtherComp :type "PrimitiveComponent Object Reference") (NormalImpulse :type "Vector Structure") (Hit :type "HitResult Structure (by ref)"))
  (`/Engine/EditorBlueprintResources/StandardMacros.IsValid` OtherActor
    (:`Is Valid`
      (`self.OnHit` OtherActor OtherComp Hit))))

(fn `OnAnyDamage`
  (params (DamagedActor :type "Actor Object Reference") (Damage :type "Float (single-precision)") (DamageType :type "DamageType Object Reference") (InstigatedBy :type "Controller Object Reference") (DamageCauser :type "Actor Object Reference"))
  (locals (NewHP :type Integer) (ResultDamage :type Integer))
  (bind _returnvalue (`HPComponent.CalcDamage` (`self.HPComp`) DamagedActor Damage DamageType InstigatedBy DamageCauser))
  (bind _returnvalue_2 (`HPComponent.SetHP` (`self.HPComp`) (- (`HPComponent.HP` (`self.HPComp`)) _returnvalue)))
  (if (and (`BlueprintGameplayTagLibrary.HasTag` (`/Game/GNG/Core/Components/BP_GravityComponent.GameplayTagContainer` (`self.BP_GravityComponent`)) (struct :`TagName` "Gravity.Hovering") true) (== (`local.DamageCauser`) (`GameplayStatics.GetPlayerCharacter` 0)))
    (`/Game/GNG/Core/Components/BP_GravityComponent.HitDetected` (`self.BP_GravityComponent`) (`KismetMathLibrary.GetRightVector` (`SceneComponent.RelativeRotation` (`Character.Mesh` (`GameplayStatics.GetPlayerCharacter` 0))))))
  (if _returnvalue_2
    _))

(fn `OnHit`
  (params (OtherActor :type "Actor Object Reference") (OtherComp :type "PrimitiveComponent Object Reference") (Hit :type "HitResult Structure (by ref)"))
  (locals (CommComponent :type "/Game/GNG/Core/Components/BP_CommComponent Object Reference") (NewG :type "Vector Structure") (HPComponent :type "HPComponent Object Reference"))
  (bind _bp_gravitycomponent (`self.BP_GravityComponent`))
  (if (and (not (`KismetMathLibrary.Vector_IsNearlyZero` (`self.GetVelocity`))) (!= (`/Game/GNG/Core/Components/BP_GravityComponent.GravityDir` _bp_gravitycomponent) (`/Game/GNG/Core/Components/BP_GravityComponent.DefaultGravityDir` _bp_gravitycomponent) :`ErrorTolerance` 0.01))
    (`ActorComponent.Deactivate` (`self.Niagara`))
    (set `local.NewG` (* (`.Normal` (`GameplayStatics.BreakHitResult` (`local.Hit`))) -1))
    (if (and (`/Game/GNG/Core/Components/BP_GravityComponent.IsWalkableSurface` (`self.BP_GravityComponent`) (`PrimitiveComponent.GetCollisionProfileName` (`local.OtherComp`)) (`local.NewG`)) (!= (`local.NewG`) (`/Game/GNG/Core/Components/BP_GravityComponent.GravityDir` (`self.BP_GravityComponent`)) :`ErrorTolerance` 0.01))
      ; SurfaceContact
      (`|ExecutionSequence`
        (:`then_0`
          (`/Game/GNG/Core/Components/BP_GravityComponent.ChangeGravity` (`self.BP_GravityComponent`) (`local.NewG`) false))
        (:`then_1`
          (`GameplayStatics.ApplyDamage` self (/ (`KismetMathLibrary.VSize` (`self.GetVelocity`)) (`PrimitiveComponent.GetMass` (`self.StaticMesh`))) null null "/Script/GNG.DT_Environmental")))
      (else
        (`/Engine/EditorBlueprintResources/StandardMacros.IsValid` (`self.GetComponentByClass` (`local.OtherActor`) "/Script/GNG.HPComponent")
          (:`Is Valid`
            (if (!= (`local.OtherActor`) (`GameplayStatics.GetPlayerCharacter` 0))
              (if (`BlueprintGameplayTagLibrary.HasTag` (`/Game/GNG/Core/Components/BP_GravityComponent.GameplayTagContainer` (`self.BP_GravityComponent`)) (struct :`TagName` "Gravity.Spinning") true)
                (`GameplayStatics.ApplyDamage` (`local.OtherActor`) (`/Game/GNG/Core/Components/BP_GravityComponent.SpinDmg` (`self.BP_GravityComponent`)) null self "/Script/GNG.DT_Environmental")
                (else
                  (`GameplayStatics.ApplyDamage` (`local.OtherActor`) (* (`/Game/GNG/Core/Components/BP_GravityComponent.GetVelocity` (`self.BP_GravityComponent`)) (`PrimitiveComponent.GetMass` (`self.StaticMesh`)) (`/Game/GNG/Core/Components/BP_GravityComponent.HitDamageReduceModif` (`self.BP_GravityComponent`))) null self "/Script/GNG.DT_Environmental"))))))))))

(fn `UserConstructionScript`)