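; Breakable obstacle actor that bounces physics objects and is destroyed when its HP runs out.
; An HP component, initialised from MaxHP on BeginPlay, calculates and applies incoming damage behind a re-entrancy guard, destroying the actor when SetHP returns false.
; Taking damage also resets gravity on the damage causer's BP_GravityComponent, if present.
; Mesh hits push simulating bodies with an acceleration-mode force of the normal impulse scaled by BounceFactor.
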(event `self.ReceiveBeginPlay`
  (bind _output_get (set `HPComponent.MAX_HP` (`self.MaxHP`) (`self.HP`)))
  (`HPComponent.SetHP` (`self.HP`) _output_get)
  (add `self.OnTakeAnyDamage` (`|CreateDelegate` :!event `OnAnyDamage`)))

(event `self.StaticMesh.OnComponentHit`
  (params (HitComponent :type "PrimitiveComponent Object Reference") (OtherActor :type "Actor Object Reference") (OtherComp :type "PrimitiveComponent Object Reference") (NormalImpulse :type "Vector Structure") (Hit :type "HitResult Structure (by ref)"))
  (`/Engine/EditorBlueprintResources/StandardMacros.IsValid` OtherComp
    (:`Is Valid`
      (if (`SceneComponent.IsSimulatingPhysics` OtherComp "None")
        (`PrimitiveComponent.AddForce` OtherComp (* NormalImpulse (`self.BounceFactor`)) "None" true)))))

(fn `OnAnyDamage`
  (params (DamagedActor :type "Actor Object Reference") (Damage :type "Float (single-precision)") (DamageType :type "DamageType Object Reference") (InstigatedBy :type "Controller Object Reference") (DamageCauser :type "Actor Object Reference"))
  (bind _hp (`self.HP`))
  (bind _returnvalue (`self.GetComponentByClass` (`local.DamageCauser`) "/Game/GNG/Core/Components/BP_GravityComponent.BP_GravityComponent_C"))
  (if (not (`self.bIsTakingDamage`))
    (set `self.bIsTakingDamage` true)
    (`/Engine/EditorBlueprintResources/StandardMacros.IsValid` _returnvalue
      (:`Is Valid`
        (`/Game/GNG/Core/Components/BP_GravityComponent.ResetGravity` _returnvalue))
      (:`Is Not Valid`
        _))
    (bind _returnvalue_2 (`HPComponent.CalcDamage` (`self.HP`) (`local.DamagedActor`) (`local.Damage`) (`local.DamageType`) (`local.InstigatedBy`) (`local.DamageCauser`)))
    (bind _returnvalue_3 (`HPComponent.SetHP` _hp (- (`HPComponent.HP` _hp) _returnvalue_2)))
    (if _returnvalue_3
      (set `self.bIsTakingDamage` false)
      (else
        (`self.K2_DestroyActor`)))))

(fn `UserConstructionScript`)