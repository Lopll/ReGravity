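; Bandit enemy character driven by BP_BanditController, with randomized health, damage, attack distance and attack montages.
; Controller states set walk speed and facing, turning it toward the player in combat, where montage hits damage the overlapped target.
; Gravity hovering switches it to flying ragdoll; capsule impacts then either land it on walkable surfaces or deal environmental damage.
; Damage updates HP, tints the material, plays reaction montages, and forwards player hits while hovering to the gravity component.
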(event `self.ReceiveBeginPlay`
  (`|ExecutionSequence`
    (:`then_0`
      (bind _asbp_bandit_controller (cast `/Game/GNG/Core/AI/BP_BanditController` (`self.GetController`)))
      (set `self.BanditController` _asbp_bandit_controller)
      (`self.DefineAttackSet`))
    (:`then_1`
      (if (`self.bActive`)
        (`self.Activate`)
        (`/Game/GNG/Core/AI/BP_BanditController.SetAttackDistance` (`self.BanditController`) (`self.AttackDistance`))))))

(event `self.ReceiveTick`
  (params (DeltaSeconds :type "Float (single-precision)"))
  (bind (_returnvalue_roll _returnvalue_pitch) (`KismetMathLibrary.BreakRotator` (`self.K2_GetActorRotation`)))
  (bind (_returnvalue_roll_2 _returnvalue_pitch_2 _returnvalue_yaw) (`KismetMathLibrary.BreakRotator` (`KismetMathLibrary.FindLookAtRotation` (`self.K2_GetActorLocation`) (`self.K2_GetActorLocation` (`GameplayStatics.GetPlayerCharacter` 0)))))
  ; RotateToPlayerIfFighting
  (if (not (`self.bUseControllerRotationYaw`))
    (`SceneComponent.K2_SetWorldRotation` (`self.CapsuleComponent`) (`KismetMathLibrary.MakeRotator` _returnvalue_roll _returnvalue_pitch _returnvalue_yaw) true false)))

(event `PlayAnim`
  (params (MontageToPlay :type "AnimMontage Object Reference"))
  (bind _banditcontroller (`self.BanditController`))
  (set `self.tempState` (cast `/Game/GNG/Core/Data/E_BanditStates` (`BlackboardComponent.GetValueAsEnum` (`AIBlueprintHelperLibrary.GetBlackboard` _banditcontroller) (`/Game/GNG/Core/AI/BP_BanditController.nState` _banditcontroller))))
  (`/Game/GNG/Core/AI/BP_BanditController.SetState` (`self.BanditController`) "NewEnumerator3")
  (`|PlayMontage` (`self.Mesh`) MontageToPlay
    (:`OnCompleted`
      (`/Game/GNG/Core/AI/BP_BanditController.SetState` (`self.BanditController`) (`self.tempState`)))))

(event `/Game/GNG/Core/Interfaces/BPI_GravityChangable.ApplyForce`
  (params (PhysComponent :type "PrimitiveComponent Object Reference") (ForceDirection :type "Vector Structure") (ForceStrength :type "Float (double-precision)") (DeltaTime :type "Float (double-precision)"))
  (`CharacterMovementComponent.AddForce` (`self.CharacterMovement`) (* ForceDirection ForceStrength)))

(event `/Game/GNG/Core/Interfaces/BPI_GravityChangable.ApplyForceAtLocalLocation`
  (params (PhysComponent :type "PrimitiveComponent Object Reference") (ForceDirection :type "Vector Structure") (ForceStrength :type "Float (double-precision)") (LocalLocation :type "Vector Structure"))
  (`CharacterMovementComponent.AddForce` (`self.CharacterMovement`) (* ForceDirection ForceStrength)))

(event `/Game/GNG/Core/Interfaces/BPI_GravityChangable.OnHoverStart`
  (bind _banditcontroller (`self.BanditController`))
  (set `self.BeforeHoverState` (cast `/Game/GNG/Core/Data/E_BanditStates` (`BlackboardComponent.GetValueAsEnum` (`AIBlueprintHelperLibrary.GetBlackboard` _banditcontroller) (`/Game/GNG/Core/AI/BP_BanditController.nState` _banditcontroller))))
  (`CharacterMovementComponent.SetMovementMode` (`self.CharacterMovement`) "MOVE_Flying" 0)
  (`/Game/GNG/Core/AI/BP_BanditController.SetState` (`self.BanditController`) "NewEnumerator1")
  (`RagdollComponent.enableRagdoll` (`self.Ragdoll`))
  (`ActorComponent.Activate` (`self.Niagara`) false))

(event `/Game/GNG/Core/Interfaces/BPI_GravityChangable.OnHoverEnd`
  (`ActorComponent.Deactivate` (`self.Niagara`))
  (`RagdollComponent.disableRagdoll` (`self.Ragdoll`))
  (`/Game/GNG/Core/AI/BP_BanditController.SetState` (`self.BanditController`) (`self.BeforeHoverState`))
  (switch `/Game/GNG/Core/Data/E_BanditStates` (`self.BeforeHoverState`)
    (:`NewEnumerator0`
      (`CharacterMovementComponent.SetMovementMode` (`self.CharacterMovement`) "MOVE_Walking" 0 :!label _label))
    (:`NewEnumerator1`
      (`CharacterMovementComponent.SetMovementMode` (`self.CharacterMovement`) "MOVE_Flying" 0))
    (:`NewEnumerator2`
      (goto _label))))

(event `/Game/GNG/Core/Interfaces/BPI_GravityChangable.AddTorque`
  (params (Torque :type "Vector Structure") (AccelChange :type Boolean))
  (`PrimitiveComponent.AddTorqueInDegrees` (`self.Mesh`) (* Torque 1000) "None" AccelChange))

(event `self.CapsuleComponent.OnComponentHit`
  (params (HitComponent :type "PrimitiveComponent Object Reference") (OtherActor :type "Actor Object Reference") (OtherComp :type "PrimitiveComponent Object Reference") (NormalImpulse :type "Vector Structure") (Hit :type "HitResult Structure (by ref)"))
  (`self.OnCapsuleComponentHit` OtherActor OtherComp (* (`.Normal` (`GameplayStatics.BreakHitResult` Hit)) -1)))

(event `ApplyDamageFromHit`
  (if (and (`|EnumEquality` (`self.State`) "NewEnumerator2") (`KismetSystemLibrary.IsValid` (`self.HitTarget`)))
    (`GameplayStatics.ApplyDamage` (`self.HitTarget`) (`self.BaseCombatDamage`) (`self.BanditController`) self "/Script/GNG.DT_Actor")
    (`GameplayStatics.PlaySoundAtLocation` (`self.HitSound`) (`self.K2_GetActorLocation`) (struct) 1.0 1.0 0.0 null null null null)))

(event `self.DMG_Box.OnComponentBeginOverlap`
  (params (OverlappedComponent :type "PrimitiveComponent Object Reference") (OtherActor :type "Actor Object Reference") (OtherComp :type "PrimitiveComponent Object Reference") (OtherBodyIndex :type Integer) (bFromSweep :type Boolean) (SweepResult :type "HitResult Structure (by ref)"))
  (set `self.HitTarget` OtherActor))

(event `self.DMG_Box.OnComponentEndOverlap`
  (params (OverlappedComponent :type "PrimitiveComponent Object Reference") (OtherActor :type "Actor Object Reference") (OtherComp :type "PrimitiveComponent Object Reference") (OtherBodyIndex :type Integer))
  (set `self.HitTarget` null))

(event `/Game/GNG/Core/Interfaces/BPI_AI_Implementable.SetState`
  (params (State :type "/Game/GNG/Core/Data/E_BanditStates Enum" :default "NewEnumerator0"))
  (bind _output_get (set `self.State` State))
  (switch `/Game/GNG/Core/Data/E_BanditStates` _output_get
    (:`NewEnumerator0`
      (set `self.bUseControllerRotationYaw` true :!label _label)
      (set `CharacterMovementComponent.MaxWalkSpeed` (`self.NormalWalkSpeed`) (`self.CharacterMovement`)))
    (:`NewEnumerator1`
      (goto _label))
    (:`NewEnumerator2`
      (set `self.bUseControllerRotationYaw` false)
      (set `CharacterMovementComponent.MaxWalkSpeed` (`self.CombatWalkSpeed`) (`self.CharacterMovement`)))
    (:`NewEnumerator3`
      (goto _label))))

(event `/Game/GNG/Core/Interfaces/BPI_AI_Implementable.PerformHit`
  (bind _attackset (`self.AttackSet`))
  (`|PlayMontage` (`self.Mesh`) (`|GetArrayItem` _attackset (`KismetMathLibrary.RandomInteger` (`KismetArrayLibrary.Array_Length` _attackset)))))

(event `/Game/GNG/Core/Interfaces/BPI_AI_Implementable.Activation`
  (set `self.bActive` true)
  (`self.Activate`))

(event `/Game/GNG/Core/Interfaces/BPI_AI_Implementable.ResetAttackDistance`
  (`/Game/GNG/Core/AI/BP_BanditController.SetAttackDistance` (`self.BanditController`) (`self.AttackDistance`)))

(fn `Activate`
  (bind _spawnpoint (`self.SpawnPoint`))
  (`|ExecutionSequence`
    (:`then_0`
      (`/Engine/EditorBlueprintResources/StandardMacros.IsValid` _spawnpoint
        (:`Is Valid`
          (`self.K2_SetActorLocation` (`self.K2_GetActorLocation` _spawnpoint) false true))))
    (:`then_1`
      (`/Engine/EditorBlueprintResources/StandardMacros.IsValid` (`self.MoveTarget`)
        (:`Is Valid`
          (`/Game/GNG/Core/AI/BP_BanditController.SetPatrolPoint` (`self.BanditController`) (`self.K2_GetActorLocation` (`self.MoveTarget`))))
        (:`Is Not Valid`
          (`/Game/GNG/Core/AI/BP_BanditController.SetPatrolPoint` (`self.BanditController`) (`self.K2_GetActorLocation`)))))))

(fn `Death`
  (`self.K2_DestroyActor`))

(fn `DefineAttackSet`
  (bind _attacks (`self.Attacks`))
  (for _ (range 3)
    (`KismetArrayLibrary.Array_Add` (`self.AttackSet`) (`|GetArrayItem` _attacks (`KismetMathLibrary.RandomInteger` (`KismetArrayLibrary.Array_Length` _attacks))))))

(fn `HitReactionEnd`)

(fn `OnAnyDamage`
  (params (DamagedActor :type "Actor Object Reference") (Damage :type "Float (single-precision)") (DamageType :type "DamageType Object Reference") (InstigatedBy :type "Controller Object Reference") (DamageCauser :type "Actor Object Reference"))
  (locals (IsAlive :type Boolean :default false))
  (bind _hp (`self.HP`))
  (if (> (`HPComponent.HP` (`self.HP`)) 0)
    (`|ExecutionSequence`
      (:`then_0`
        (bind _returnvalue (`HPComponent.CalcDamage` (`self.HP`) (`local.DamagedActor`) (`local.Damage`) (`local.DamageType`) (`local.InstigatedBy`) (`local.DamageCauser`)))
        (bind _returnvalue_2 (`HPComponent.SetHP` _hp (- (`HPComponent.HP` _hp) _returnvalue)))
        (set `local.IsAlive` _returnvalue_2)
        (`self.SetMaterialColorToHP`))
      (:`then_1`
        (if (and (`BlueprintGameplayTagLibrary.HasTag` (`/Game/GNG/Core/Components/BP_GravityComponent.GameplayTagContainer` (`self.BP_GravityComponent`)) (struct :`TagName` "Gravity.Hovering") true) (== (`local.DamageCauser`) (`GameplayStatics.GetPlayerCharacter` 0)))
          (`/Game/GNG/Core/Components/BP_GravityComponent.HitDetected` (`self.BP_GravityComponent`) (`KismetMathLibrary.GetRightVector` (`SceneComponent.RelativeRotation` (`Character.Mesh` (`GameplayStatics.GetPlayerCharacter` 0)))))))
      (:`then_2`
        (if (`local.IsAlive`)
          (`self.PlayAnim` (`self.DamageAnim`))
          (else
            (`self.PlayAnim` (`self.DeathAnim`))))))))

(fn `OnCapsuleComponentHit`
  (params (OtherActor :type "Actor Object Reference") (OtherComp :type "PrimitiveComponent Object Reference") (NewGDirection :type "Vector Structure"))
  (bind _bp_gravitycomponent (`self.BP_GravityComponent`))
  (`/Engine/EditorBlueprintResources/StandardMacros.IsValid` OtherActor
    (:`Is Valid`
      (if (!= (`/Game/GNG/Core/Components/BP_GravityComponent.GravityDir` _bp_gravitycomponent) (`/Game/GNG/Core/Components/BP_GravityComponent.DefaultGravityDir` _bp_gravitycomponent) :`ErrorTolerance` 0.01)
        (if (and (`|EnumEquality` (`CharacterMovementComponent.MovementMode` (`self.CharacterMovement`)) "MOVE_Flying") (`/Game/GNG/Core/Components/BP_GravityComponent.IsWalkableSurface` (`self.BP_GravityComponent`) (`PrimitiveComponent.GetCollisionProfileName` (`local.OtherComp`)) (`local.NewGDirection`)))
          (`self.SetGravityToSurface` (`local.NewGDirection`))
          (else
            (`/Engine/EditorBlueprintResources/StandardMacros.IsValid` (`self.GetComponentByClass` (`local.OtherActor`) "/Script/GNG.HPComponent")
              (:`Is Valid`
                (if (!= (`local.OtherActor`) (`GameplayStatics.GetPlayerCharacter` 0))
                  (if (`BlueprintGameplayTagLibrary.HasTag` (`/Game/GNG/Core/Components/BP_GravityComponent.GameplayTagContainer` (`self.BP_GravityComponent`)) (struct :`TagName` "Gravity.Spinning") true)
                    (`GameplayStatics.ApplyDamage` (`local.OtherActor`) (`/Game/GNG/Core/Components/BP_GravityComponent.SpinDmg` (`self.BP_GravityComponent`)) null self "/Script/GNG.DT_Environmental")
                    (elif (!= (`GameplayStatics.GetObjectClass` (`local.OtherActor`)) (`GameplayStatics.GetObjectClass` self))
                      (`GameplayStatics.ApplyDamage` (`local.OtherActor`) (* (`/Game/GNG/Core/Components/BP_GravityComponent.GetVelocity` (`self.BP_GravityComponent`)) (`self.Mass`) (`/Game/GNG/Core/Components/BP_GravityComponent.HitDamageReduceModif` (`self.BP_GravityComponent`))) null self "/Script/GNG.DT_Environmental"))))))))))))

(fn `SetGravityToSurface`
  (params (NewGDirection :type "Vector Structure"))
  (`/Game/GNG/Core/Components/BP_GravityComponent.ResetGravity` (`self.BP_GravityComponent`))
  (`RagdollComponent.disableRagdoll` (`self.Ragdoll`))
  (`CharacterMovementComponent.SetMovementMode` (`self.CharacterMovement`) "MOVE_Walking" 0)
  (`/Game/GNG/Core/AI/BP_BanditController.SetState` (`self.BanditController`) "NewEnumerator0")
  (if (not (== (`/Game/GNG/Core/Components/BP_GravityComponent.DefaultGravityDir` (`self.BP_GravityComponent`)) (`local.NewGDirection`)))
    (`GameplayStatics.ApplyDamage` self (/ (`KismetMathLibrary.VSize` (`self.GetVelocity`)) (`self.Mass`)) null null "/Script/GNG.DT_Environmental")))

(fn `SetMaterialColorToHP`
  (locals (Material :type "MaterialInstanceDynamic Object Reference") (Perc :type "Float (double-precision)"))
  (bind _perc (`local.Perc`))
  (bind _hp (`self.HP`))
  (set `local.Perc` (/ (`KismetMathLibrary.Conv_IntToDouble` (`HPComponent.HP` _hp)) (`KismetMathLibrary.Conv_IntToDouble` (`HPComponent.MAX_HP` _hp))))
  (bind _returnvalue (`PrimitiveComponent.CreateDynamicMaterialInstance` (`self.Mesh`) 0 (`PrimitiveComponent.GetMaterial` (`self.Mesh`) 0) "None"))
  (bind _output_get (set `local.Material` _returnvalue))
  (bind _returnvalue_2 (`MaterialInstanceDynamic.K2_GetVectorParameterValue` _output_get "Color"))
  (`MaterialInstanceDynamic.SetVectorParameterValue` (`local.Material`) "Color" (make `LinearColor` (break `LinearColor` _returnvalue_2) _perc _perc (`.A` (break `LinearColor` _returnvalue_2))))
  (bind _returnvalue_3 (`MaterialInstanceDynamic.K2_GetVectorParameterValue` (`local.Material`) "Emiss_Color"))
  (bind (_h _s _v _a) (`KismetMathLibrary.RGBToHSV` _returnvalue_3))
  (`MaterialInstanceDynamic.SetVectorParameterValue` (`local.Material`) "Emiss_Color" (`KismetMathLibrary.HSVToRGB` _h _s (`local.Perc`) _a))
  (`PrimitiveComponent.SetMaterial` (`self.Mesh`) 0 (`local.Material`)))

(fn `UserConstructionScript`
  (bind _bp_gravitycomponent (`self.BP_GravityComponent`))
  (bind _hp (`self.HP`))
  (set `/Game/GNG/Core/Components/BP_GravityComponent.PhysicBase` (`self.CapsuleComponent`) _bp_gravitycomponent)
  (set `/Game/GNG/Core/Components/BP_GravityComponent.MeshComponent` (`self.Mesh`) _bp_gravitycomponent)
  (bind _output_get (set `self.MAX_HP` (+ (`KismetMathLibrary.RandomInteger` 41) 70)))
  (bind _output_get_2 (set `HPComponent.MAX_HP` _output_get _hp))
  (`HPComponent.SetHP` _hp _output_get_2)
  (add `self.OnTakeAnyDamage` (`|CreateDelegate` :!event `OnAnyDamage`))
  (set `self.BaseCombatDamage` (/ (`self.MAX_HP`) 6))
  (set `self.AttackDistance` (`KismetMathLibrary.Conv_IntToDouble` (`KismetMathLibrary.RandomIntegerInRange` 250 600))))