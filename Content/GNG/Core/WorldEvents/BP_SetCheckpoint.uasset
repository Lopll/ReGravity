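; BP_SetCheckpoint is a one-shot world checkpoint with an animated mesh that visibly activates when triggered.
; The first box overlap passes the sweep result location to the player character's SetCheckpoint, without checking which actor overlapped.
; It also switches the mesh from a looping pose to a looping dance and yellow lamp material, plays a sound and activates two Niagara effects.
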(event `self.ReceiveBeginPlay`
  (`SkeletalMeshComponent.PlayAnimation` (`self.SkeletalMesh`) "/Game/GNG/Animation/Bandit/Female_Dynamic_Pose.Female_Dynamic_Pose" true))

(event `self.Box.OnComponentBeginOverlap`
  (params (OverlappedComponent :type "PrimitiveComponent Object Reference") (OtherActor :type "Actor Object Reference") (OtherComp :type "PrimitiveComponent Object Reference") (OtherBodyIndex :type Integer) (bFromSweep :type Boolean) (SweepResult :type "HitResult Structure (by ref)"))
  (bind _asbp_player_character (cast `/Game/GNG/Core/Player/BP_PlayerCharacter` (`GameplayStatics.GetPlayerCharacter` 0)))
  (`/Engine/EditorBlueprintResources/StandardMacros.DoOnce` false
    (:`Completed`
      (`/Game/GNG/Core/Player/BP_PlayerCharacter.SetCheckpoint` _asbp_player_character (`.Location` (`GameplayStatics.BreakHitResult` SweepResult)))
      (`SkeletalMeshComponent.PlayAnimation` (`self.SkeletalMesh`) "/Game/GNG/Animation/Silly_Dancing.Silly_Dancing" true)
      (`PrimitiveComponent.SetMaterial` (`self.SkeletalMesh`) 0 "/Game/GNG/Materials/M_YellowLamp.M_YellowLamp")
      (`GameplayStatics.PlaySoundAtLocation` (`self.ActivationSound`) (`self.K2_GetActorLocation`) (struct) 1.0 1.0 0.0 null null null null)
      (`ActorComponent.Activate` (`self.Niagara`) false)
      (`ActorComponent.Activate` (`self.Niagara1`) false))))

(fn `UserConstructionScript`
  (`parent.UserConstructionScript`))