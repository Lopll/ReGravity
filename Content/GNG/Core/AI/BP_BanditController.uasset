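; AI controller for bandit enemies that runs BT_Bandit and switches the pawn between states as it senses or loses the player.
; Perception updates set the combat target, move target and state in the blackboard, and Tick refreshes the target's location while fighting.
; A lost player is only dropped beyond a set distance, making that stimulus location the patrol point.
; SetState also notifies the pawn and disables perception handling in one state.
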(event `self.ReceiveBeginPlay`)

(event `self.ReceivePossess`
  (params (PossessedPawn :type "Pawn Object Reference"))
  (set `self.Possessed Pawn` PossessedPawn)
  (`self.RunBehaviorTree` "/Game/GNG/Core/AI/BT_Bandit.BT_Bandit"))

(event `self.ReceiveTick`
  (params (DeltaSeconds :type "Float (single-precision)"))
  (if (`self.bFighting`)
    (`BlackboardComponent.SetValueAsVector` (`AIBlueprintHelperLibrary.GetBlackboard` null) (`self.nCombatTargetLocation`) (`self.K2_GetActorLocation` (`self.CombatTarget`)))))

(event `self.AIPerception.OnTargetPerceptionInfoUpdated`
  (params (UpdateInfo :type "ActorPerceptionUpdateInfo Structure (by ref)"))
  (if (`self.bPerceptionActive`)
    (`self.OnTargetPerceptionInfoUpdated` UpdateInfo)))

(fn `OnTargetPerceptionInfoUpdated`
  (params (ActorPerceptionUpdateInfo :type "ActorPerceptionUpdateInfo Structure (by ref)"))
  (locals (Stimulus :type "AIStimulus Structure"))
  (bind (_targetid _target _stimulus) (break `ActorPerceptionUpdateInfo` ActorPerceptionUpdateInfo))
  (bind (_targetid_2 _target_2 _stimulus_2) (break `ActorPerceptionUpdateInfo` (`local.ActorPerceptionUpdateInfo`)))
  (bind (_age _expirationage _strength _stimuluslocation _receiverlocation) (break `AIStimulus` (`local.Stimulus`)))
  (if (== (`GameplayStatics.GetPlayerCharacter` 0) _target)
    (set `local.Stimulus` _stimulus)
    (if (`.bSuccessfullySensed` (break `AIStimulus` (`local.Stimulus`)))
      (`BlackboardComponent.SetValueAsObject` (`AIBlueprintHelperLibrary.GetBlackboard` null) (`self.nCombatTarget`) _target_2)
      (set `self.CombatTarget` _target_2)
      (`BlackboardComponent.SetValueAsVector` (`AIBlueprintHelperLibrary.GetBlackboard` null) (`self.nCombatTargetLocation`) (`self.K2_GetActorLocation` (`self.CombatTarget`)))
      (`self.SetMoveTarget` (`.StimulusLocation` (break `AIStimulus` _stimulus_2)))
      (`self.SetState` "NewEnumerator2")
      (set `self.bFighting` true)
      (elif (>= (`KismetMathLibrary.VSize` (- _stimuluslocation _receiverlocation)) 1100.0)
        (`BlackboardComponent.SetValueAsObject` (`AIBlueprintHelperLibrary.GetBlackboard` null) (`self.nCombatTarget`) null)
        (`self.SetState` "NewEnumerator0")
        (`self.SetPatrolPoint` (`.StimulusLocation` (break `AIStimulus` (`local.Stimulus`))))
        (set `self.bFighting` false)
        (set `self.CombatTarget` null)))))

(fn `SetAttackDistance`
  (params (AttackDistance :type "Float (double-precision)"))
  (`BlackboardComponent.SetValueAsFloat` (`AIBlueprintHelperLibrary.GetBlackboard` null) (`self.nAttackDistance`) AttackDistance))

(fn `SetMoveTarget`
  (params (MoveTarget :type "Vector Structure"))
  (`BlackboardComponent.SetValueAsVector` (`AIBlueprintHelperLibrary.GetBlackboard` null) (`self.nMoveTarget`) (`local.MoveTarget`)))

(fn `SetPatrolPoint`
  (params (PatrolPoint :type "Vector Structure"))
  (`BlackboardComponent.SetValueAsVector` (`AIBlueprintHelperLibrary.GetBlackboard` null) (`self.nPatrolPoint`) (`local.PatrolPoint`)))

(fn `SetState`
  (params (State :type "/Game/GNG/Core/Data/E_BanditStates Enum" :default "NewEnumerator0"))
  (`BlackboardComponent.SetValueAsEnum` (`AIBlueprintHelperLibrary.GetBlackboard` null) (`self.nState`) (`local.State`))
  (message `/Game/GNG/Core/Interfaces/BPI_AI_Implementable.SetState` (`self.Possessed Pawn`) (`local.State`))
  (if (`|EnumEquality` (`local.State`) "NewEnumerator1")
    (set `self.bPerceptionActive` false)
    (else
      (set `self.bPerceptionActive` true)
      (if (and (`|EnumEquality` (`local.State`) "NewEnumerator0") (`KismetSystemLibrary.IsValid` (`self.CombatTarget`)))
        (`self.SetState` "NewEnumerator2")))))

(fn `UserConstructionScript`)